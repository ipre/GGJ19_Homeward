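; Upgrade pickup that unlocks one of the player's abilities (Move, Jump, Swim, Dash or Fly) when interacted with.
; The construction script picks the Cube component's mesh from UpgradeType, so each placed instance shows the matching item.
; On interaction it enables that upgrade on the PC_Homeward player controller, makes the mesh visible, calls CreateWidget and destroys itself.
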(event `/Game/HomeWard/Blueprints/I_HomewardInteraction.InteractWith`
  (bind _aspc_homeward (cast `/Game/HomeWard/Blueprints/PC_Homeward` (`GameplayStatics.GetPlayerController` 0)))
  (`/Game/HomeWard/Blueprints/PC_Homeward.setUpgrade` _aspc_homeward (`self.UpgradeType`) true)
  (`SceneComponent.SetVisibility` (`self.Cube`) true false)
  (`|CreateWidget` null)
  (`self.K2_DestroyActor`))

(fn `UserConstructionScript`
  (bind _cube (`self.Cube`))
  (`parent.UserConstructionScript`)
  (switch `/Game/HomeWard/Blueprints/Enum_Upgrade` (`self.UpgradeType`)
    (:`NewEnumerator0`
      (`StaticMeshComponent.SetStaticMesh` _cube "/Game/HomeWard/Character/Home/Item_Legs.Item_Legs"))
    (:`NewEnumerator1`
      (`StaticMeshComponent.SetStaticMesh` _cube "/Game/HomeWard/Character/Home/Item_Springs.Item_Springs"))
    (:`NewEnumerator2`
      (`StaticMeshComponent.SetStaticMesh` _cube "/Game/HomeWard/Character/Home/Item_Swim.Item_Swim"))
    (:`NewEnumerator3`
      (`StaticMeshComponent.SetStaticMesh` _cube "/Game/HomeWard/Character/Home/Item_Rammon.Item_Rammon"))
    (:`NewEnumerator4`
      (`StaticMeshComponent.SetStaticMesh` _cube "/Game/HomeWard/Character/Home/Item_Wings.Item_Wings"))))