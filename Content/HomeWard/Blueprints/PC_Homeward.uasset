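; PC_Homeward is the Homeward player controller, judging by its prefix, and stores which movement upgrades are unlocked: Move, Jump, Swim, Dash and Fly.
; Each upgrade is a boolean, read or written by type through switches in HasUpgrade and SetUpgrade.
; GetUpgrade returns all flags at once.
; BeginPlay only prints a test string, and the file contains no movement logic.
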(event `self.ReceiveBeginPlay`
  (`KismetSystemLibrary.PrintString` "testsetset"))

(fn `GetUpgrade`
  (returns (Move :type Boolean) (Jump :type Boolean) (Swim :type Boolean) (Dash :type Boolean) (Fly :type Boolean))
  (return (`self.hasMove`) (`self.hasJump`) (`self.hasSwim`) (`self.hasDash`) (`self.hasFly`)))

(fn `hasUpgrade`
  (params (UpgradeType :type "/Game/HomeWard/Blueprints/Enum_Upgrade Enum" :default "NewEnumerator0"))
  (returns (Bool :type Boolean))
  (switch `/Game/HomeWard/Blueprints/Enum_Upgrade` UpgradeType
    (:`NewEnumerator0`
      (return (`self.hasMove`)))
    (:`NewEnumerator1`
      (return (`self.hasJump`)))
    (:`NewEnumerator2`
      (return (`self.hasSwim`)))
    (:`NewEnumerator3`
      (return (`self.hasDash`)))
    (:`NewEnumerator4`
      (return (`self.hasFly`)))))

(fn `setUpgrade`
  (params (Upgradetype :type "/Game/HomeWard/Blueprints/Enum_Upgrade Enum" :default "NewEnumerator0") (NewState :type Boolean :default true))
  (switch `/Game/HomeWard/Blueprints/Enum_Upgrade` Upgradetype
    (:`NewEnumerator0`
      (set `self.hasMove` NewState))
    (:`NewEnumerator1`
      (set `self.hasJump` NewState))
    (:`NewEnumerator2`
      (set `self.hasSwim` NewState))
    (:`NewEnumerator3`
      (set `self.hasDash` NewState))
    (:`NewEnumerator4`
      (set `self.hasFly` NewState)))
  (return))

(fn `UserConstructionScript`)