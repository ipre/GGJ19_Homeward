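; BP_IK_Test is a test actor that computes ground-contact data for foot IK on a skeletal mesh.
; Each Tick, IKFootTrace casts a Visibility line down from actor height at each foot socket's XY.
; Offset is the distance between trace end and hit location, smoothed with FInterpTo into LeftOffset and RightOffset.
; Raw hit locations go to LeftLoc and RightLoc, with no check for a missed trace.
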(event `self.ReceiveTick`
  (params (DeltaSeconds :type "Float (single-precision)"))
  (bind (_offset _location) (`self.IKFootTrace` 150.0 "L_FootSocket"))
  (set `self.LeftLoc` _location)
  (set `self.LeftOffset` (`KismetMathLibrary.FInterpTo` (`self.LeftOffset`) _offset DeltaSeconds 1.3))
  (bind (_offset_2 _location_2) (`self.IKFootTrace` 150.0 "R_FootSocket"))
  (set `self.RightLoc` _location_2)
  (set `self.RightOffset` (`KismetMathLibrary.FInterpTo` (`self.RightOffset`) _offset_2 DeltaSeconds 1.3)))

(fn `IKFootTrace`
  (params (Trace :type "Float (double-precision)") (Name :type Name))
  (returns (Offset :type "Float (double-precision)") (Location :type "Vector Structure"))
  (bind (_returnvalue_x _returnvalue_y _returnvalue_z) (`KismetMathLibrary.BreakVector` (`self.K2_GetActorLocation`)))
  (bind (_returnvalue_x_2 _returnvalue_y_2) (`KismetMathLibrary.BreakVector` (`SceneComponent.GetSocketLocation` (`self.SkeletalMesh`) Name)))
  (bind _returnvalue (`KismetMathLibrary.MakeVector` _returnvalue_x_2 _returnvalue_y_2 (- _returnvalue_z Trace)))
  (bind (_outhit _returnvalue_2) (`KismetSystemLibrary.LineTraceSingle` (`KismetMathLibrary.MakeVector` _returnvalue_x_2 _returnvalue_y_2 _returnvalue_z) _returnvalue "TraceTypeQuery1"))
  (bind (_bblockinghit _binitialoverlap _time _distance _location) (`GameplayStatics.BreakHitResult` _outhit))
  (return (`KismetMathLibrary.VSize` (- _returnvalue _location)) _location))

(fn `UserConstructionScript`)